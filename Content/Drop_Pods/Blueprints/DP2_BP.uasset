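; Drop pod actor that handles the effects, sounds and animations of a falling and landing pod.
; Tick watches CurrentDropProgress, opening engines and firing thrusters halfway down, then cutting them near the ground, with timelines fading thruster and wind audio.
; DropPodLanded plays the impact sound and chains timers to close engines, then open the door.
; Construction script sets floor visibility and door variant, and snaps thrusters to engine sockets.
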(event Custom|Close%20Engines
  ;[1 1 1] Close engines shortly after landing
  (Components|Animation|PlayAnimation (Variables|Default|GetDrop_Mesh) "/Game/Drop_Pods/Anims/DP2_Close_Anim.DP2_Close_Anim" false)
  (Utilities|Time|SetTimerbyEvent (delegate Custom|Open%20Pod) 1.0))

(event Custom|Open%20Pod
  ;[1 1 1] Open door, shortly after landing
  (Components|Animation|PlayAnimation (Variables|Default|GetDoor) (select (Variables|Default|GetDoor%201) "/Game/Drop_Pods/Anims/DP2_Lid1_Open1_Anim.DP2_Lid1_Open1_Anim" "/Game/Drop_Pods/Anims/DP2_lid2_Open_Anim.DP2_lid2_Open_Anim") false))

(event EventBeginPlay
  (|CallParentFunction))

(event EventTick
  (params (DeltaSeconds :type Float%20%28single-precision%29))
  (bind _thruster_2 (Variables|Default|GetThruster_2))
  ;[1 1 1] Is drop progress over walf way through falling?
  (|CallParentFunction DeltaSeconds)
  (if (<= (Variables|Default|GetCurrent%20Drop%20Progress) 0.5)
    (Utilities|FlowControl|Sequence
      (:then_0
        (Utilities|FlowControl|DoOnce false
          (:Completed
            ;[1 1 1] Activate and deactivate thruster effects
            (Components|Animation|PlayAnimation (Variables|Default|GetDrop_Mesh) "/Game/Drop_Pods/Anims/DP2_Open_Anim.DP2_Open_Anim" false)
            (Utilities|FlowControl|Delay 0.07)
            (Rendering|SetVisibility _thruster_2 true false)
            (Components|Activation|Activate _thruster_2 false)
            (bind (_direction _volume) (Timeline|Thruster%20Sound PlayFromStart)
              (:Update
                (Audio|Components|Audio|SetVolumeMultiplier (Variables|Default|GetThruster_Sound) _volume :!class /Script/Engine.AudioComponent))
              (:Finished
                (switch Utilities|FlowControl|Switch|SwitchonETimelineDirection _direction
                  (:Forward
                    ;[1 1 1] End falling wind sound after thrusters fire and drop pod slows down
                    (bind _volume_2 (Timeline|Wind%20Fade%20Out PlayFromStart)
                      (:Update
                        (Audio|Components|Audio|SetVolumeMultiplier (Variables|Default|GetWind%20Sound) _volume_2 :!class /Script/Engine.AudioComponent))))))))))
      (:then_1
        ;[1 1 1] Is drop progress almost entireley through falling?
        (if (<= (Variables|Default|GetCurrent%20Drop%20Progress) 0.08)
          (Utilities|FlowControl|DoOnce false
            (:Completed
              (Components|Activation|Deactivate (Variables|Default|GetThruster_2))
              (Timeline|Thruster%20Sound ReverseFromEnd))))))))

(event EventDropPodLanded
  (bind _hit_sound (Variables|Default|GetHit%20Sound))
  (Utilities|Time|SetTimerbyEvent (delegate Custom|Close%20Engines) 1.0)
  ;[1 1 1] Play sound when landing
  (Audio|Components|Audio|Play _hit_sound 0.0)
  (bind _volume (Timeline|Play%20the%20lounding%20sound PlayFromStart)
    (:Update
      (Audio|Components|Audio|SetVolumeMultiplier _hit_sound _volume :!class /Script/Engine.AudioComponent))))

(fn ConstructionScript
  (bind _drop_mesh (Variables|Default|GetDrop_Mesh))
  ;[1 1 1] Set initial door and floor values
  (|CallParentFunction)
  (Rendering|SetVisibility (Variables|Default|GetFloor) (Variables|Default|GetHas%20Floor) false)
  (Components|SkinnedMesh|SetSkinnedAssetandUpdate (Variables|Default|GetDoor) (select (Variables|Default|GetDoor%201) "/Game/Drop_Pods/Meshes/DP2_Lid1_SK.DP2_Lid1_SK" "/Game/Drop_Pods/Meshes/DP2_lid2_SK.DP2_lid2_SK") true)
  ;[1 1 1] Set thrusters to engine sockets
  (Transformation|AttachComponentToComponent (Variables|Default|GetThruster_1) _drop_mesh "engine_1Socket" "SnapToTarget" "SnapToTarget" "KeepRelative" true)
  (Transformation|AttachComponentToComponent (Variables|Default|GetThruster_2) _drop_mesh "engine_2Socket" "SnapToTarget" "SnapToTarget" "KeepRelative" true)
  (Transformation|AttachComponentToComponent (Variables|Default|GetThruster_3) _drop_mesh "engine_3Socket" "SnapToTarget" "SnapToTarget" "KeepRelative" true)
  (Transformation|AttachComponentToComponent (Variables|Default|GetThruster_4) _drop_mesh "engine_4Socket" "SnapToTarget" "SnapToTarget" "KeepRelative" true))