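; Drop pod actor that handles the landing sequence once the pod reaches the end of its spline path.
; DropPodLanded traces vertically to attach a crack decal to the hit actor, while timelines drive the wind and impact sound volumes.
; Chained timers close the fins by playing the break animation in reverse, then play the door-opening animation.
; The construction script poses the mesh in that break animation beforehand.
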(event Custom|Close%20Fins
  (bind _drop_mesh (Variables|Default|GetDrop_Mesh))
  ;[1 1 1] Close the fins
  (Components|Animation|PlayAnimation _drop_mesh "/Game/Drop_Pods/Anims/DP1_Open_Break_Anim.DP1_Open_Break_Anim" false)
  (Components|Animation|SetPosition _drop_mesh 0.398 false)
  (Components|Timeline|SetPlayRate _drop_mesh -0.3)
  (Utilities|Time|SetTimerbyEvent (delegate Custom|Open%20Pod) 1.4))

(event Custom|Open%20Pod
  ;[1 1 1] Open the door
  (Components|Animation|PlayAnimation (Variables|Default|GetDrop_Mesh) "/Game/Drop_Pods/Anims/DP1_Open1_Anim.DP1_Open1_Anim" false))

(event EventBeginPlay
  (|CallParentFunction))

(event EventTick
  (params (DeltaSeconds :type Float%20%28single-precision%29))
  (|CallParentFunction DeltaSeconds))

(event EventDropPodLanded
  (bind _returnvalue (Transformation|GetActorLocation))
  (bind _hit_sound (Variables|Default|GetHit%20Sound))
  ;[1 1 1] Event when the end of the spline path was reached
  (Utilities|Time|SetTimerbyEvent (delegate Custom|Close%20Fins) 2.2)
  ;[1 1 1] Add an impact decal
  (bind _outhit (Collision|LineTraceByChannel (+ _returnvalue "0, 0,500.000000") (+ _returnvalue "0, 0,-500.000000") "TraceTypeQuery1" false 0 "None"))
  (bind _returnvalue_2 (AddComponent|AddDecalComponent (.hitactor _outhit) false (Class|KismetMathLibrary|ConvertTransformtoRelative (Transformation|GetActorTransform (.hitactor _outhit)) (Math|Transform|MakeTransform (.location _outhit) (Math|Rotator|MakeRotfromX (.normal _outhit)) "0.200000,1,1.000000"))))
  (Rendering|Components|Decal|SetDecalMaterial _returnvalue_2 "/Game/Drop_Pods/Materials/Cracks_M.Cracks_M")
  ;[1 1 1] Stop the blowing wind sound and play an impact effect upon landing
  (Utilities|FlowControl|Sequence
    (:then_0
      (bind _volume (Timeline|End%20Wind%20Sound PlayFromStart)
        (:Update
          (Audio|Components|Audio|SetVolumeMultiplier (Variables|Default|GetWind%20Sound) _volume :!class /Script/Engine.AudioComponent))))
    (:then_1
      (Audio|Components|Audio|Play _hit_sound 0.0)
      (bind _volume_2 (Timeline|Play%20Hit%20Sound PlayFromStart)
        (:Update
          (Audio|Components|Audio|SetVolumeMultiplier _hit_sound _volume_2 :!class /Script/Engine.AudioComponent))))))

(fn ConstructionScript
  (|CallParentFunction)
  (Components|Animation|OverrideAnimationData (Variables|Default|GetDrop_Mesh) "/Game/Drop_Pods/Anims/DP1_Open_Break_Anim.DP1_Open_Break_Anim" false false 1.0 1.0))