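; Master drop pod actor that falls along an editable spline over a set drop time, then lands with effects and sound.
; Tick counts down the timer, using curves to drive spline position and mesh twist.
; Landing fires a message for child Blueprints and optionally traces the surface, easing the mesh to its normal via a timeline.
; Landed's OnRep forces the final update; the construction script previews placement along the spline.
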(event Custom|Man%20Update%20Drop
  (bind _drop_location (Variables|Default|GetDrop%20Location))
  (bind _drop_path (Variables|Default|GetDrop_Path))
  (bind _drop_location_2 (Variables|Default|GetDrop%20Location))
  (bind _drop_mesh (Variables|Default|GetDrop_Mesh))
  (bind _returnvalue (Transformation|GetWorldLocation _drop_location))
  (bind _returnvalue_2 (Spline|GetSplineLength _drop_path))
  (bind _returnvalue_3 (Transformation|GetWorldLocation _drop_location_2))
  (bind _returnvalue_4 (Transformation|GetWorldRotation _drop_mesh))
  (bind _returnvalue_5 (Math|Vector|GetRightVector _returnvalue_4))
  ;[1 1 1] Cound down the current drop time, and set the current drop progress value
  (bind _output_get (Variables|Default|SetCurrent%20Drop%20Time (Math|Float|Clamp(Float) (- (Variables|Default|GetCurrent%20Drop%20Time) (stale EventTick DeltaSeconds)) 0.0 (Variables|Default|GetDrop%20Time))))
  (bind _output_get_2 (Variables|Default|SetCurrent%20Drop%20Progress (/ _output_get (Variables|Default|GetDrop%20Time))))
  ;[1 1 1] Set the drop locations transform to match a given point along the drop path based on the current drop progress
  (Transformation|SetWorldTransform (Variables|Default|GetDrop%20Location) (Spline|GetTransformatDistanceAlongSpline _drop_path (- _returnvalue_2 (* _returnvalue_2 (Math|Curves|GetFloatValue (Variables|Default|GetDrop%20Progress%20Curve) _output_get_2))) "World" true) false false)
  ;[1 1 1] Give the mesh some rotaiton as it falls
  (Transformation|AddLocalRotation (Variables|Default|GetDrop_Mesh) (Math|Rotator|MakeRotator 0.0 0.0 (* (Math|Curves|GetFloatValue (Variables|Default|GetDrop%20Twist%20Curve) (Variables|Default|GetCurrent%20Drop%20Progress)) (Utilities|Time|GetWorldDeltaSeconds))) false false)
  ;[1 1 1] If drop time equals 0, then trigger landing effects and set landed to true
  (if (== (Variables|Default|GetCurrent%20Drop%20Time) 0.0)
    (Utilities|FlowControl|DoOnce false
      (:Completed
        (Variables|Default|SetLanded true)
        (Effects|SpawnEmitteratLocation (Variables|Default|GetLanding%20Effect) _returnvalue_3 (Math|Conversions|RotationFromXVector (Math|Vector|GetUpVector _drop_location_2)))
        (Audio|PlaySoundatLocation (Variables|Default|GetLanding%20Sound) _returnvalue_3 "0, 0, 0" 1.0 1.0 0.0 0 0 0 0)
        ;[1 1 1] Send message for DP landing, used in child actors for custom events
        (Class|DropPodBPI|DropPodLanded(Message) self)
        ;[1 1 1] Look at the surface the DP hit, and orient it to that surface. If you have noisy/bumpy surfaces on the visual side, with smoother/consistent collision surfaces, then set it to trace the collision one in most cases, nothing like a drop pod being on its side because it hit a pebble.
        (if (Variables|Default|GetOrient%20To%20Surface%20Normal%20On%20Landing)
          (bind _outhit (Collision|LineTraceByChannel (+ _returnvalue "0, 0,300.000000") (+ _returnvalue "0, 0,-300.000000") "TraceTypeQuery1" false 0 "None"))
          (Variables|Default|SetInitial%20Rotation (Transformation|GetWorldRotation (Variables|Default|GetDrop_Mesh)))
          (Variables|Default|SetTarget%20Rotation (Math|Rotator|MakeRotationfromAxes (Math|Vector|CrossProduct _returnvalue_5 (.normal _outhit)) _returnvalue_5 (.normal _outhit)))
          (bind _lerp (Timeline|Lerp%20To%20Surface%20Normal PlayFromStart)
            (:Update
              (Transformation|SetWorldRotation (Variables|Default|GetDrop_Mesh) (Math|Rotator|Lerp(Rotator) (Variables|Default|GetInitial%20Rotation) (Variables|Default|GetTarget%20Rotation) _lerp true) false false))))))))

(event EventBeginPlay
  ;[1 1 1] Set the current drop time to the total drop time at start of play
  (Variables|Default|SetCurrent%20Drop%20Time (Variables|Default|GetDrop%20Time)))

(event EventTick
  (params (DeltaSeconds :type Float%20%28single-precision%29))
  (bind _drop_location (Variables|Default|GetDrop%20Location))
  (bind _drop_path (Variables|Default|GetDrop_Path))
  (bind _drop_location_2 (Variables|Default|GetDrop%20Location))
  (bind _drop_mesh (Variables|Default|GetDrop_Mesh))
  (bind _returnvalue (Transformation|GetWorldLocation _drop_location))
  (bind _returnvalue_2 (Spline|GetSplineLength _drop_path))
  (bind _returnvalue_3 (Transformation|GetWorldLocation _drop_location_2))
  (bind _returnvalue_4 (Transformation|GetWorldRotation _drop_mesh))
  (bind _returnvalue_5 (Math|Vector|GetRightVector _returnvalue_4))
  ;[1 1 1] Cound down the current drop time, and set the current drop progress value
  (if (not (Variables|Default|GetLanded))
    (bind _output_get (Variables|Default|SetCurrent%20Drop%20Time (Math|Float|Clamp(Float) (- (Variables|Default|GetCurrent%20Drop%20Time) DeltaSeconds) 0.0 (Variables|Default|GetDrop%20Time))))
    (bind _output_get_2 (Variables|Default|SetCurrent%20Drop%20Progress (/ _output_get (Variables|Default|GetDrop%20Time))))
    ;[1 1 1] Set the drop locations transform to match a given point along the drop path based on the current drop progress
    (Transformation|SetWorldTransform (Variables|Default|GetDrop%20Location) (Spline|GetTransformatDistanceAlongSpline _drop_path (- _returnvalue_2 (* _returnvalue_2 (Math|Curves|GetFloatValue (Variables|Default|GetDrop%20Progress%20Curve) _output_get_2))) "World" true) false false)
    ;[1 1 1] Give the mesh some rotaiton as it falls
    (Transformation|AddLocalRotation (Variables|Default|GetDrop_Mesh) (Math|Rotator|MakeRotator 0.0 0.0 (* (Math|Curves|GetFloatValue (Variables|Default|GetDrop%20Twist%20Curve) (Variables|Default|GetCurrent%20Drop%20Progress)) (Utilities|Time|GetWorldDeltaSeconds))) false false)
    ;[1 1 1] If drop time equals 0, then trigger landing effects and set landed to true
    (if (== (Variables|Default|GetCurrent%20Drop%20Time) 0.0)
      (Utilities|FlowControl|DoOnce false
        (:Completed
          (Variables|Default|SetLanded true)
          (Effects|SpawnEmitteratLocation (Variables|Default|GetLanding%20Effect) _returnvalue_3 (Math|Conversions|RotationFromXVector (Math|Vector|GetUpVector _drop_location_2)))
          (Audio|PlaySoundatLocation (Variables|Default|GetLanding%20Sound) _returnvalue_3 "0, 0, 0" 1.0 1.0 0.0 0 0 0 0)
          ;[1 1 1] Send message for DP landing, used in child actors for custom events
          (Class|DropPodBPI|DropPodLanded(Message) self)
          ;[1 1 1] Look at the surface the DP hit, and orient it to that surface. If you have noisy/bumpy surfaces on the visual side, with smoother/consistent collision surfaces, then set it to trace the collision one in most cases, nothing like a drop pod being on its side because it hit a pebble.
          (if (Variables|Default|GetOrient%20To%20Surface%20Normal%20On%20Landing)
            (bind _outhit (Collision|LineTraceByChannel (+ _returnvalue "0, 0,300.000000") (+ _returnvalue "0, 0,-300.000000") "TraceTypeQuery1" false 0 "None"))
            (Variables|Default|SetInitial%20Rotation (Transformation|GetWorldRotation (Variables|Default|GetDrop_Mesh)))
            (Variables|Default|SetTarget%20Rotation (Math|Rotator|MakeRotationfromAxes (Math|Vector|CrossProduct _returnvalue_5 (.normal _outhit)) _returnvalue_5 (.normal _outhit)))
            (bind _lerp (Timeline|Lerp%20To%20Surface%20Normal PlayFromStart)
              (:Update
                (Transformation|SetWorldRotation (Variables|Default|GetDrop_Mesh) (Math|Rotator|Lerp(Rotator) (Variables|Default|GetInitial%20Rotation) (Variables|Default|GetTarget%20Rotation) _lerp true) false false)))))))))

(fn ConstructionScript
  (bind _drop_path (Variables|Default|GetDrop_Path))
  ;[1 1 1] Set initial preview position along the drop spline, such as at the end of it where it would land, and the drop meshes transform value
  (Transformation|SetWorldTransform (Variables|Default|GetDrop%20Location) (Spline|GetTransformatDistanceAlongSpline _drop_path (* (Spline|GetSplineLength _drop_path) (Variables|Default|GetPreview%20Spline%20Lerp)) "World" false) false false)
  (Transformation|SetRelativeTransform (Variables|Default|GetDrop_Mesh) (Variables|Default|GetSet%20Mesh%20Initial%20Relative%20Transform) false false))

(fn OnRepLanded
  (Variables|Default|SetCurrent%20Drop%20Time 0.0)
  (CallFunction|ManUpdateDrop))