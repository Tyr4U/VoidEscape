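; Drop pod variant that descends along a spline, optionally carrying the player, and either lands and opens or bursts apart mid-air.
; On landing it closes airbrakes, plays an opening animation, projects a crack decal and crossfades wind to impact audio.
; When exploding, it swaps to a breakable physics asset near the spline's end, scatters parts by impulse and despawns later.
; A dropped player possesses the child actor, then a spawned character upon bursting.
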(event Custom|Open%20Pod
  (bind _drop_mesh (Variables|Default|GetDrop_Mesh))
  ;[1 1 1] Open door/s
  (if (Variables|Default|GetUse%20Open%20Anim%201)
    (Components|Animation|PlayAnimation _drop_mesh "/Game/Drop_Pods/Anims/DP3_Open1_Anim.DP3_Open1_Anim" false)
    (else
      (Components|Animation|PlayAnimation _drop_mesh "/Game/Drop_Pods/Anims/DP3_Open2_Anim.DP3_Open2_Anim" false))))

(event Custom|Despawn%20Old%20Bits
  ;[1 1 1] After 10 seconds, destroy the actor to clean up its various parts
  (Actor|DestroyActor))

(event EventBeginPlay
  (bind _returnvalue (Game|GetPlayerController 0))
  ;[1 1 1] If set to drop player, then possess the newly spawned drop pod
  (|CallParentFunction)
  (if (Variables|Default|GetDrop%20Player)
    (Pawn|UnPossess _returnvalue)
    (Pawn|Possess _returnvalue (.AsPawn (Utilities|Casting|CastToPawn (Variables|/Script/Engine.ChildActorComponent|GetChildActor (Variables|Default|GetChildActor)))))))

(event EventTick
  (params (DeltaSeconds :type Float%20%28single-precision%29))
  (bind _returnvalue (Game|GetPlayerController 0))
  (bind _drop_mesh (Variables|Default|GetDrop_Mesh))
  ;[1 1 1] If the drop pod should explode open while dropping in mid air, find when its near the bottom of its drop spline, and then trigger the parts to break apart
  (|CallParentFunction DeltaSeconds)
  (if (Variables|Default|GetExplode%20On%20Drop)
    (if (<= (Variables|Default|GetCurrent%20Drop%20Progress) 0.05)
      (Utilities|FlowControl|DoOnce false
        (:Completed
          (Variables|Default|SetLanded true)
          ;[1 1 1] If dropping the player, spawn a pawn for them in the drop pod as it bursts open and possess it.
          (if (Variables|Default|GetDrop%20Player)
            (bind _returnvalue_2 (Game|SpawnActorfromClass "/Game/Drop_Pods/Third_Person_Content/ThirdPersonBP/Blueprints/ThirdPersonCharacter.ThirdPersonCharacter_C" (Math|Conversions|ToTransform(Vector) (Transformation|GetSocketLocation (Variables|Default|GetDrop_Mesh) "player_location")) "AlwaysSpawn" 0 0))
            (Pawn|UnPossess _returnvalue)
            (Pawn|Possess _returnvalue _returnvalue_2))
          ;[1 1 1] Change the physics asset to the one where the parts aren't held together, enable physics simulation, and then add an impulse to send the parts flying apart
          (Components|SkinnedMesh|SetPhysicsAsset _drop_mesh "/Game/Drop_Pods/Meshes/DP3_Explodable_PhysicsAsset.DP3_Explodable_PhysicsAsset" false)
          (Physics|SetSimulatePhysics _drop_mesh true)
          (Class|SkeletalMeshComponent|AddImpulsetoAllBodiesBelow _drop_mesh "0,0.000000,-5000.000000" "root_dr3" true false)
          ;[1 1 1] Stop the wind blowing sound as the actor bursts in the air.
          (bind _volume (Timeline|Stop%20Wind PlayFromStart)
            (:Update
              (Audio|Components|Audio|SetVolumeMultiplier (Variables|Default|GetWind_Sound) _volume :!class /Script/Engine.AudioComponent))
            (:Finished
              ;[1 1 1] After 10 seconds, destroy the actor to clean up its various parts
              (Utilities|Time|SetTimerbyEvent (delegate Custom|Despawn%20Old%20Bits) 1e+01))))))))

(event EventDropPodLanded
  (bind _returnvalue (Transformation|GetActorLocation))
  (bind _hit_sound (Variables|Default|GetHit%20Sound))
  ;[1 1 1] Close airbrakes after drop pod reaches the end of its descent spline
  (Components|Animation|PlayAnimation (Variables|Default|GetDrop_Mesh) "/Game/Drop_Pods/Anims/DP3_Airbrake_Close_Anim.DP3_Airbrake_Close_Anim" false)
  (Utilities|Time|SetTimerbyEvent (delegate Custom|Open%20Pod) 1.0)
  ;[1 1 1] Add an impact decal
  (bind _outhit (Collision|LineTraceByChannel (+ _returnvalue "0, 0,500.000000") (+ _returnvalue "0, 0,-500.000000") "TraceTypeQuery1" false 0 "None"))
  (bind _returnvalue_2 (AddComponent|AddDecalComponent (.hitactor _outhit) false (Class|KismetMathLibrary|ConvertTransformtoRelative (Transformation|GetActorTransform (.hitactor _outhit)) (Math|Transform|MakeTransform (.location _outhit) (Math|Rotator|MakeRotfromX (.normal _outhit)) "0.150000,2.000000,2.000000"))))
  (Rendering|Components|Decal|SetDecalMaterial _returnvalue_2 "/Game/Drop_Pods/Materials/Cracks_M.Cracks_M")
  ;[1 1 1] When landing, stop the wind blowing sound, and play a hit sound
  (Utilities|FlowControl|Sequence
    (:then_0
      (bind _volume (Timeline|End%20Wind%20Sound PlayFromStart)
        (:Update
          (Audio|Components|Audio|SetVolumeMultiplier (Variables|Default|GetWind_Sound) _volume :!class /Script/Engine.AudioComponent))))
    (:then_1
      (Audio|Components|Audio|Play _hit_sound 0.0)
      (bind _volume_2 (Timeline|Produce%20Hit%20Sound PlayFromStart)
        (:Update
          (Audio|Components|Audio|SetVolumeMultiplier _hit_sound _volume_2 :!class /Script/Engine.AudioComponent))))))

(fn ConstructionScript
  (bind _drop_mesh (Variables|Default|GetDrop_Mesh))
  ;[1 1 1] Set some initial values, like animation, and collision resonses before play
  (|CallParentFunction)
  (Components|Animation|OverrideAnimationData (Variables|Default|GetDrop_Mesh) "/Game/Drop_Pods/Anims/DP3_Airbrake_Loop_Anim.DP3_Airbrake_Loop_Anim" true true 0.0 1.0)
  (if (Variables|Default|GetExplode%20On%20Drop)
    (Collision|SetCollisionResponsetoChannel _drop_mesh "ECC_Pawn" "ECR_Ignore")
    (Collision|SetCollisionResponsetoChannel _drop_mesh "ECC_PhysicsBody" "ECR_Ignore")
    (else
      (Collision|SetCollisionResponsetoChannel _drop_mesh "ECC_Pawn" "ECR_Block")
      (Collision|SetCollisionResponsetoChannel _drop_mesh "ECC_PhysicsBody" "ECR_Block")))
  (Variables|Default|SetOrient%20To%20Surface%20Normal%20On%20Landing (Variables|Default|GetLevel%20Actor%20On%20Landing)))