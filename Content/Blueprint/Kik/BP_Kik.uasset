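; Kik player character with health, sprint, jetpack fuel and effects, and win/lose events.
; Interact input messages overlapping BPI_Interact actors, sending pickup on press and guzzle while triggered.
; Fuel helpers drain by delta time, clamp refills and report percentage; refills and game results go to the cached player controller for UI.
; Thruster start/stop events toggle twin visuals and sounds, reusing one attached looping audio component rather than respawning it.
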(event Custom|KixsHealth
  (bind _bpc_health (Variables|Default|GetBPC_Health))
  ;[0.2308 1 0.1369] Player Health
  (Variables|/Game/Blueprint/Blueprints/Components/BPC_Health.BPC_Health_C|SetCurrentHealth _bpc_health (Variables|/Game/Blueprint/Blueprints/Components/BPC_Health.BPC_Health_C|GetMaxHealth _bpc_health)))

(event Custom|CurrentJetFuel
  ;[0.2308 1 0.1369] Set Jet Fuel Player Starts With
  (Variables|JetFuel|SetCurrentFuel (Variables|JetFuel|GetCurrentFuel)))

(event Input|EnhancedActionEvents|EnhancedInputActionIA_Sprint
  (params (ActionValue :type Boolean) (ElapsedSeconds :type Float%20%28double-precision%29) (TriggeredSeconds :type Float%20%28double-precision%29) (InputAction :type Input%20Action%20Object%20Reference :default "/Game/Input/IA_Sprint.IA_Sprint"))
  (bind _charactermovement (Variables|Character|GetCharacterMovement))
  ;[0.1666 0.9901 1] Handle Sprint
  (:Started
    (Variables|/Script/Engine.CharacterMovementComponent|SetMaxWalkSpeed _charactermovement 6e+02))
  (:Completed
    (Variables|/Script/Engine.CharacterMovementComponent|SetMaxWalkSpeed _charactermovement 3e+02)))

(event Input|EnhancedActionEvents|EnhancedInputActionIA_Interact
  (params (ActionValue :type Boolean) (ElapsedSeconds :type Float%20%28double-precision%29) (TriggeredSeconds :type Float%20%28double-precision%29) (InputAction :type Input%20Action%20Object%20Reference :default "/Game/Input/IA_Interact.IA_Interact"))
  ;[0.1666 0.9901 1] Interact with objects in the world
  (:Triggered
    (bind _array_element (Utilities|Array|ForEachLoopwithBreak (Collision|GetOverlappingActors "/Script/Engine.Actor" :!class /Script/Engine.Actor))
      (:LoopBody
        (if (Utilities|DoesObjectImplementInterface _array_element "/Game/Blueprint/Blueprints/Interfaces/BPI_Interact.BPI_Interact_C")
          (Class|BPIInteract|Guzzle(Message) _array_element)))))
  (:Started
    (bind _array_element_2 (Utilities|Array|ForEachLoopwithBreak (Collision|GetOverlappingActors "/Script/Engine.Actor" :!class /Script/Engine.Actor))
      (:LoopBody
        (if (Utilities|DoesObjectImplementInterface _array_element_2 "/Game/Blueprint/Blueprints/Interfaces/BPI_Interact.BPI_Interact_C")
          (Class|BPIInteract|Pickup(Message) _array_element_2))))))

(event EventBeginPlay
  ;[0.3802 0.3802 0.3802] Event Begin Play Events
  (CallFunction|Referances)
  (CallFunction|KixsHealth)
  (CallFunction|CurrentJetFuel))

(event EventStopThruster
  ;[0.1666 0.9901 1] Activate and Deactivate Jetpack Thrusters ON Interface
  (JetPack|ActivateThrusterVisuals false)
  (JetPack|StopThrusterSound))

(event EventStartThruster
  ;[0.1666 0.9901 1] Activate and Deactivate Jetpack Thrusters ON Interface
  (JetPack|ActivateThrusterVisuals true)
  (JetPack|StartThrusterSound))

(event EventWinGame
  ;[0.2308 1 0.1369] Win and Lost states and Events
  (bind _as_bp_kix_player_controller_base (Variables|Default|GetAs%20BP%20Kix%20Player%20Controller%20Base)
    (:then
      (Default|ShowEndGameWidget _as_bp_kix_player_controller_base true))
    (:else)))

(event EventLoseGame
  ;[0.2308 1 0.1369] Win and Lost states and Events
  (bind _as_bp_kix_player_controller_base (Variables|Default|GetAs%20BP%20Kix%20Player%20Controller%20Base)
    (:then
      (Default|ShowEndGameWidget _as_bp_kix_player_controller_base false))
    (:else)))

(event EventRefillFuel
  (params (FuelAmount :type Float%20%28double-precision%29))
  ;[0.2308 1 0.1369] Refill the Jetpack on Pickup
  (CallFunction|HandleRefillFuel FuelAmount))

(fn ConstructionScript)

(fn Referances
  ;[0.1666 0.9901 1] Player Controller
  (bind _asbp_kix_player_controller_base (Utilities|Casting|CastToBP_KixPlayerController_Base (Pawn|GetController)))
  (Variables|Default|SetAs%20BP%20Kix%20Player%20Controller%20Base _asbp_kix_player_controller_base))

(fn StartThrusterSound
  ;[0.1666 0.9901 1] Handle Start of Jetpack Sound
  (bind _returnvalue (Audio|SpawnSoundatLocation "/Game/Assets/Sounds/Thrusters/MS_ThrusterStart.MS_ThrusterStart" (Transformation|GetActorLocation) "0, 0, 0" 1.0 1.0 0.0 0 0))
  (Audio|Components|Audio|FadeOut _returnvalue 1.0 0.0 "Linear" :!class /Script/Engine.AudioComponent)
  (Utilities|IsValid (Variables|Thrusters|GetLoopingThrusterSound)
    (:Is%20Valid
      ;;[0 0.06699 1] More performant to avoid memory leak
      ;;;[0 0 0] Play IF IsValid?
      (Audio|Components|Audio|Play (Variables|Thrusters|GetLoopingThrusterSound) 0.0)
      (Audio|Components|Audio|FadeIn (Variables|Thrusters|GetLoopingThrusterSound) 0.35 1.0 0.0 "Linear" :!class /Script/Engine.AudioComponent))
    (:Is%20Not%20Valid
      ;;;[0 0 0] Start Thruster Sound for The First Time IF IsNOTvalid?
      (bind _returnvalue_2 (Audio|SpawnSoundAttached "/Game/Assets/Sounds/Thrusters/MS_ThrusterLoop.MS_ThrusterLoop" (Variables|Collision|GetCapsuleComponent) "None" "0, 0, 0" "0, 0, 0" "KeepRelativeOffset" false 0.6 1.0 0.0 0 0))
      (bind _output_get (Variables|Thrusters|SetLoopingThrusterSound _returnvalue_2))
      (Audio|Components|Audio|FadeIn _output_get 0.35 1.0 0.0 "Linear" :!class /Script/Engine.AudioComponent))))

(fn StopThrusterSound
  ;[0.1666 0.9901 1] Handle STOP Thruster Sound
  (bind _loopingthrustersound (Variables|Thrusters|GetLoopingThrusterSound)
    (:then
      (Audio|Components|Audio|Stop _loopingthrustersound)
      (bind _returnvalue (Audio|SpawnSoundatLocation "/Game/Assets/Sounds/Thrusters/MS_ThrusterStop.MS_ThrusterStop" (Transformation|GetActorLocation) "0, 0, 0" 0.4 1.0 0.0 0 0))
      (Audio|Components|Audio|FadeOut _returnvalue 0.55 0.0 "Linear" :!class /Script/Engine.AudioComponent))
    (:else)))

(fn ActivateThrusterVisuals
  (params (Activate :type Boolean))
  ;[0.1666 0.9901 1] Check Thruster Visuals
  (if Activate
    (Components|Activation|Activate (Variables|Default|GetThruster_R) false)
    (else
      (Components|Activation|Deactivate (Variables|Default|GetThruster_R)))))

(fn JetFuelDrainPerFrame
  ;[0.1666 0.9901 1] Set Jet Fuel to a Clamped Value by - Jet Fuel by the Sum of Jet Fuyel Drain Rate * World Delta Sec
  (Variables|JetFuel|SetCurrentFuel (Math|Float|Clamp(Float) (- (Variables|JetFuel|GetCurrentFuel) (* (Variables|JetFuel|GetJetFuelDrainRate) (Utilities|Time|GetWorldDeltaSeconds))) 0.0 (Variables|JetFuel|GetMaxJetFuel))))

(fn FuelPercent
  ;[0.1666 0.9901 1] Send Fuel Percentage
  (return (Math|Float|SafeDivide (Variables|JetFuel|GetCurrentFuel) (Variables|JetFuel|GetMaxJetFuel))))

(fn HandleRefillFuel
  (params (FuelAmount :type Float%20%28double-precision%29))
  ;[0.2308 1 0.1369] Add Jet Fuel to Current Jet Fuel Via Pickup
  (Variables|JetFuel|SetCurrentFuel (Math|Float|Clamp(Float) (+ FuelAmount (Variables|JetFuel|GetCurrentFuel)) 0.0 (Variables|JetFuel|GetMaxJetFuel)))
  (bind _as_bp_kix_player_controller_base (Variables|Default|GetAs%20BP%20Kix%20Player%20Controller%20Base)
    (:then
      (Default|FuelUpdate _as_bp_kix_player_controller_base (CallFunction|FuelPercent)))
    (:else)))

(fn GetCenterSizeBox
  (params (EndGameWidget :type WBP%20End%20Game%20Object%20Reference))
  (bind _returnvalue (Viewport|GetViewportSize))
  (bind _sizebox_root (Variables|/Game/Blueprint/Blueprints/Widget/WBP_EndGame.WBP_EndGame_C|GetSizeBox_Root EndGameWidget))
  (return (Math|Vector2D|MakeVector2D (- (/ (.x _returnvalue) 2.0) (/ (Variables|/Script/UMG.SizeBox|GetWidthOverride _sizebox_root) 2.0)) (- (/ (.y _returnvalue) 4.0) (/ (Variables|/Script/UMG.SizeBox|GetHeightOverride _sizebox_root) 2.0)))))

(fn DrainJetFuel
  ;[0.2308 1 0.1369] Get Jetfuel Percentage
  (JetFuel|JetFuelDrainPerFrame)
  (return (CallFunction|FuelPercent)))

(fn GetActionInput
  ;[0.2308 1 0.1369] Get Action Value of Kixs
  (return (Input|EnhancedActionValues|GetIA_Movement)))

(fn HasFuel
  ;[0.2308 1 0.1369] Has Jet Fuel above 0
  (return (> (Variables|JetFuel|GetCurrentFuel) 0.0)))

(fn NoFuel
  (return false))