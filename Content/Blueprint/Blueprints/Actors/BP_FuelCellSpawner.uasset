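; BP_FuelCellSpawner is an actor that keeps spawning floating fuel cell pickups around its location.
; On BeginPlay it starts a looping timer on SpawnTime, and each tick of that timer spawns one BP_Pickup_FuelCell_Floating with a random rotation.
; GetRandomPointInSphereRadius picks each position by scaling a random rotator's forward vector by a random distance up to Radius, so points cluster toward the center.
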(event Custom|SpawnFuelCells
  ;[0.1666 0.9901 1] Spawn Fuel Cell Timer on Event Begin Play
  (Game|SpawnActorfromClass "/Game/Blueprint/Blueprints/Actors/Pickups/BP_Pickup_FuelCell_Floating.BP_Pickup_FuelCell_Floating_C" (Math|Transform|MakeTransform (CallFunction|GetRandomPointinSphereRadius) (Math|Random|RandomRotator false) "1.000000,1.000000,1.000000") "Undefined" "MultiplyWithRoot" 0 0))

(event EventBeginPlay
  ;[0.1666 0.9901 1] Spawn Fuel Cell Timer on Event Begin Play
  (Utilities|Time|SetTimerbyEvent (delegate Custom|SpawnFuelCells) (Variables|Default|GetSpawnTime) true))

(fn ConstructionScript)

(fn GetRandomPointinSphereRadius
  ;[0.2308 1 0.1369] Calculate Random point by + Actor Location and Forward Vector of the Rotator * Sphere Radius of 250 in a Random Float in Range
  (return (+ (Transformation|GetActorLocation) (* (Math|Vector|GetForwardVector (Math|Random|RandomRotator false)) (Math|Random|RandomFloatinRange 0.0 (Variables|Default|GetRadius))))))