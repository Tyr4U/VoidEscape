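; BP_ScoreRing_Base is a score ring actor that awards points when something overlaps its trigger.
; The TriggerScore overlap casts the game mode to GM_KikMode and adds AddedScoreAmount to PlayerScore.
; A DoOnce with no reset limits each ring to one award, and the overlapping actor is not filtered.
; The construction script applies the Color material variable to the Ring component.
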(event OnComponentBeginOverlap(TriggerScore)
  (params (OverlappedComponent :type Primitive%20Component%20Object%20Reference) (OtherActor :type Actor%20Object%20Reference) (OtherComp :type Primitive%20Component%20Object%20Reference) (OtherBodyIndex :type Integer) (bFromSweep :type Boolean) (SweepResult :type Hit%20Result%20Structure%20%28by%20ref%29))
  ;[0.1666 0.9901 1] On overlap ADD to the Score
  (bind _asgm_kik_mode (Utilities|Casting|CastToGM_KikMode (Game|GetGameMode)))
  (Utilities|FlowControl|DoOnce false
    (:Completed
      (Variables|/Game/Blueprint/GameModes/GM_KikMode.GM_KikMode_C|SetPlayerScore _asgm_kik_mode (+ (Variables|/Game/Blueprint/GameModes/GM_KikMode.GM_KikMode_C|GetPlayerScore _asgm_kik_mode) (Variables|Default|GetAddedScoreAmount))))))

(fn ConstructionScript
  (Rendering|Material|SetMaterial (Variables|Default|GetRing) 0 (Variables|Default|GetColor)))