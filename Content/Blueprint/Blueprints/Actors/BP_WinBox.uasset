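; BP_WinBox is an actor that signals a game win when its Activate event fires.
; It checks whether the soft class reference KixClass is already valid and async-loads it if not.
; Both paths then find the first actor of that class and send it WinGameMessage, provided one exists.
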(event EventActivate
  (bind _kixclass (Variables|Default|GetKixClass))
  ;[0.1666 0.9901 1] On Activate Load Win Game IF iSValid Class? True/ On False Load Win Game for first time. BPI WinGame message recieved I
  (if (Utilities|IsValidClass (Utilities|ResolveSoftReference (Variables|Default|GetKixClass)))
    _
    (else
      ;;[0 0 0] Load for first time
      (Utilities|AsyncLoadClassAsset _kixclass
        (:Completed
          _))))
  (bind _outactors (Actor|GetAllActorsOfClass (Utilities|ResolveSoftReference _kixclass)))
  (if (Utilities|Array|IsValidIndex _outactors)
    (Class|BPIWinLose|WinGame(Message) (Utilities|Array|Get(acopy) _outactors))))

(fn ConstructionScript)