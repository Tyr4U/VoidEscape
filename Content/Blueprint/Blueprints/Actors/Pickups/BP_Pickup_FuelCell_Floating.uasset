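; Floating fuel cell pickup that drifts along its forward vector with a random spin and increments the score when a Pawn overlaps it.
; On BeginPlay it scales in via timeline, picks its rotation rate, starts a lifetime timer and binds the trigger overlap.
; Overlap increments the score once through GM_KikMode, then calls WinkOut, which the timer also fires.
; WinkOut plays a scale timeline on the mesh and destroys the actor.
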(event Custom|WinkIn
  ;[0.1666 0.9901 1] Wink into the world
  (bind _scale (Timeline|Timeline Play)
    (:Update
      (Transformation|SetWorldScale3D (Variables|Default|GetItem) _scale))))

(event Custom|WinkOut
  ;[0.3802 0.3802 0.3802] Event Begin Play
  ;;[0 0 0] WinkOut on Life of Fuel Key
  (bind _scale (Timeline|TL_Winkout Play)
    (:Update
      (CallFunction|ScaleFuelKey _scale))
    (:Finished
      (Actor|DestroyActor))))

(event Custom|OnComponentBeginOverlap_Event
  (params (OverlappedComponent :type Primitive%20Component%20Object%20Reference) (OtherActor :type Actor%20Object%20Reference) (OtherComp :type Primitive%20Component%20Object%20Reference) (OtherBodyIndex :type Integer) (bFromSweep :type Boolean) (SweepResult :type Hit%20Result%20Structure%20%28by%20ref%29))
  ;[0.3802 0.3802 0.3802] Event Begin Play
  ;;[0 0 0] When Player Overlaps Volume Wink Out
  (if (Class|GameplayStatics|ObjectIsA OtherActor "/Script/Engine.Pawn")
    (bind _asgm_kik_mode (Utilities|Casting|CastToGM_KikMode (Game|GetGameMode)))
    (Utilities|FlowControl|DoOnce false
      (:Completed
        (Default|IncrementScore _asgm_kik_mode)
        (CallFunction|WinkOut)))))

(event EventBeginPlay
  ;[0.3802 0.3802 0.3802] Event Begin Play
  (|CallParentFunction)
  (CallFunction|Winkin)
  (CallFunction|InitializeRotation)
  (Utilities|Time|SetTimerbyEvent (delegate Custom|WinkOut) (Variables|Default|GetLifetime))
  ;;[0 0 0] When Player Overlaps Volume Wink Out
  (Collision|AssignOnComponentBeginOverlap (Variables|Default|GetTriggerPickup) (delegate Custom|OnComponentBeginOverlap_Event)))

(event EventTick
  (params (DeltaSeconds :type Float%20%28single-precision%29))
  ;[0.1666 0.9901 1] Movement of Mesh per Frame
  (CallFunction|MoveandRotateActor DeltaSeconds))

(fn ConstructionScript
  (|CallParentFunction))

(fn MoveandRotateActor
  (params (DeltaTime :type Float%20%28double-precision%29))
  ;[0.1666 0.9901 1] Add Actor World Offset for Movement Speed and Direction/Add World Rotation (Rotate at Random Rotations)
  (Transformation|AddActorWorldOffset (* (Transformation|GetActorForwardVector) (* DeltaTime (Variables|Default|GetSpeed))))
  (Class|Actor|AddActorWorldRotation (* (Variables|Default|GetDeltaRotation) DeltaTime)))

(fn InitializeRotation
  ;[0.1666 0.9901 1] Rotate at Random Scale
  (Variables|Default|SetDeltaRotation (* (Math|Random|RandomRotator false) (Variables|Default|GetRotationScaleFactor))))

(fn ScaleFuelKey
  (params (Scale :type Float%20%28single-precision%29))
  (Transformation|SetWorldScale3D (Variables|Default|GetItem) (Math|Vector|MakeVector Scale Scale Scale)))