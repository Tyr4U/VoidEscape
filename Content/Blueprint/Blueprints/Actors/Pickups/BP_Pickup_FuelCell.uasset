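; BP_Pickup_FuelCell is a fuel cell pickup that refuels the overlapping actor and adds to the player's score.
; On overlap it runs the parent handler, sends RefillFuelMessage to the other actor, then plays a 2D sound and spawns the fuel pickup effect at its location.
; It then casts the game mode to GM_KikMode, increments PlayerScore and destroys itself; if that cast fails, the pickup is not destroyed.
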(event Collision|EventActorBeginOverlap
  (params (OtherActor :type Actor%20Object%20Reference))
  ;[0.3802 0.3802 0.3802] Handle overlap event for Pickup
  (|CallParentFunction OtherActor)
  (Class|BPIJetpack|RefillFuel(Message) OtherActor 0.25)
  (CallFunction|HandleEffects)
  (bind _asgm_kik_mode (Utilities|Casting|CastToGM_KikMode (Game|GetGameMode)))
  (bind _result (Math|Integer|IncrementInt (Variables|/Game/Blueprint/GameModes/GM_KikMode.GM_KikMode_C|GetPlayerScore _asgm_kik_mode))
    (:%20%20
      (Variables|/Game/Blueprint/GameModes/GM_KikMode.GM_KikMode_C|SetPlayerScore _asgm_kik_mode _result)
      (Actor|DestroyActor))))

(fn ConstructionScript
  (|CallParentFunction))

(fn HandleEffects
  (Audio|PlaySound2D "/Game/Assets/Sounds/JetFuel/SW_HexSpawn_03.SW_HexSpawn_03" 1.0 1.0 0.0 0 0)
  (Niagara|SpawnSystematLocation "/Game/Assets/Effects/JetFuel/NS_FuelPickup.NS_FuelPickup" (Transformation|GetActorLocation)))