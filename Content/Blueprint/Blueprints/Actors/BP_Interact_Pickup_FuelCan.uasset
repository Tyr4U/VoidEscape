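; Interactable jet fuel canister pickup that refills the player's fuel when picked up.
; On pickup it runs the parent logic, then a timeline tilts the item before it sends the refill message to the player, plays the fuel effect and sound, and destroys itself after a short delay.
; Overlapping the trigger toggles a popup widget for the player character only.
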(event OnComponentBeginOverlap(TriggerWidget)
  (params (OverlappedComponent :type Primitive%20Component%20Object%20Reference) (OtherActor :type Actor%20Object%20Reference) (OtherComp :type Primitive%20Component%20Object%20Reference) (OtherBodyIndex :type Integer) (bFromSweep :type Boolean) (SweepResult :type Hit%20Result%20Structure%20%28by%20ref%29))
  ;[0.1666 0.9901 1] Set visibility on Widget Popup
  (if (== OtherActor (Game|GetPlayerCharacter 0))
    (Rendering|SetVisibility (Variables|Default|GetPopup) true false)))

(event OnComponentEndOverlap(TriggerWidget)
  (params (OverlappedComponent :type Primitive%20Component%20Object%20Reference) (OtherActor :type Actor%20Object%20Reference) (OtherComp :type Primitive%20Component%20Object%20Reference) (OtherBodyIndex :type Integer))
  ;[0.1666 0.9901 1] Set visibility on Widget Popup
  (if (== OtherActor (Game|GetPlayerCharacter 0))
    (Rendering|SetVisibility (Variables|Default|GetPopup) false false)))

(event EventPickup
  ;[0.1666 0.9901 1] Handle Interact Event with a Tilt and a Sound then Destroy
  (|CallParentFunction)
  (bind _tiltjetfuelcanister (Timeline|TL_JetfuelPickup PlayFromStart)
    (:Update
      (Transformation|SetRelativeRotation (Variables|Default|GetItem) (Math|Rotator|Lerp(Rotator) "0, 0, 0" "0.000000,0.000000,45.000000" _tiltjetfuelcanister) false false))
    (:Finished
      (Class|BPIJetpack|RefillFuel(Message) (Variables|Default|GetPlayerCharacter) 0.5)
      (Components|Activation|Activate (Variables|Default|GetFuelSFX) false)
      ;;[1 0.9385 0] Fuel Gulp Sound
      (Audio|PlaySound2D "/Game/Assets/Sounds/JetFuel/SW_HexSpawn_01.SW_HexSpawn_01" 1.0 1.0 0.0 0 0)
      (Utilities|FlowControl|Delay 0.5)
      (Actor|DestroyActor))))

(event EventBeginPlay
  ;[0.3802 0.3802 0.3802] Event Begin Play
  (bind _ascharacter (Utilities|Casting|CastToCharacter (Game|Player|GetPlayerPawn 0)))
  (Variables|Default|SetPlayerCharacter _ascharacter))

(fn ConstructionScript
  (|CallParentFunction))