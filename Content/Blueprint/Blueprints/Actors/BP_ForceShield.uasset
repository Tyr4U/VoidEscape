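; BP_ForceShield is a force field actor whose material reacts to the position of the BP_Kik player.
; BeginPlay creates a dynamic material instance on the Field component, and a Sphere overlap starts and stops tracking BP_Kik.
; While tracking, Tick writes the player's world location into the PlayerPos vector parameter.
; The interface event Activate destroys the shield, while ToggleVisability is an empty stub with unconnected visibility logic.
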(event OnComponentBeginOverlap(Sphere)
  (params (OverlappedComponent :type Primitive%20Component%20Object%20Reference) (OtherActor :type Actor%20Object%20Reference) (OtherComp :type Primitive%20Component%20Object%20Reference) (OtherBodyIndex :type Integer) (bFromSweep :type Boolean) (SweepResult :type Hit%20Result%20Structure%20%28by%20ref%29))
  ;[0.1666 0.9901 1] On Sphere Overlap Event Set track Player to True
  (bind _asbp_kik (Utilities|Casting|CastToBP_Kik OtherActor))
  (Variables|Default|SetPlayerRef _asbp_kik)
  (Variables|Default|SetTrackPlayer true))

(event OnComponentEndOverlap(Sphere)
  (params (OverlappedComponent :type Primitive%20Component%20Object%20Reference) (OtherActor :type Actor%20Object%20Reference) (OtherComp :type Primitive%20Component%20Object%20Reference) (OtherBodyIndex :type Integer))
  ;[0.1666 0.9901 1] On End Overlap Set Track Player to False
  (Utilities|Casting|CastToBP_Kik OtherActor)
  (Variables|Default|SetTrackPlayer false))

(event Custom|ToggleVisability
  ;[0.1666 0.9901 1] Toggle Visibility of ForceField
)

(event EventBeginPlay
  ;[0.3802 0.3802 0.3802] Event Begin Play
  (bind _returnvalue (Rendering|Material|CreateDynamicMaterialInstance (Variables|Default|GetField) 0 "/Game/Material/MI_ForceField_ShieldShield.MI_ForceField_ShieldShield" "None" :!class /Script/Engine.PrimitiveComponent))
  (bind _output_get (Variables|Default|SetMatInst _returnvalue))
  (Rendering|Material|SetVectorParameterValue _output_get "PlayerPos" (Math|Color|MakeColor 0.0 0.0 0.0 0.0) :!class /Script/Engine.MaterialInstanceDynamic))

(event EventActivate
  ;[0.1666 0.9901 1] (BPI) On Event Activate Destroy Shield
  (Actor|DestroyActor))

(event EventTick
  (params (DeltaSeconds :type Float%20%28single-precision%29))
  (bind _playerref (Variables|Default|GetPlayerRef))
  (bind _returnvalue (Transformation|GetActorLocation _playerref))
  ;[0.1666 0.9901 1] Event Tick *IF Track Player is True give Actor the Force Field Material
  (if (Variables|Default|GetTrackPlayer)
    (Rendering|Material|SetVectorParameterValue (Variables|Default|GetMatInst) "PlayerPos" (Math|Color|MakeColor (.x _returnvalue) (.y _returnvalue) (.z _returnvalue)) :!class /Script/Engine.MaterialInstanceDynamic)))

(fn ConstructionScript)