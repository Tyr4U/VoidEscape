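; Player controller for the Kix character, handling Enhanced Input look, movement, jump and jetpack, plus camera zoom and UI.
; The jetpack switches movement to Flying, adds upward input and drains fuel through character interface messages, updating the HUD.
; Mouse wheel input sets a camera position that Tick interpolates into spring arm length.
; The end-game menu async-loads its class if needed, shows win/lose text and binds restart and quit delegates.
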(event Custom|ResetJetpack
  ;[0.1666 0.9901 1] Start Jetpack Thrusters and set Movement Mode to Flying on Started
  ;;[1 0 0] If PC Has Fuel, Apply Thrust and Drain Fuel, otherwisw Stop Jetpack
  (Utilities|FlowControl|DoOnce false) ; enters at Reset
)

(event Custom|ToggleHud
  ;[0.1666 0.9901 1] Toggle HUD On/Off
  (if (Variables|Default|GetbIsMainMenu)
    (bind _returnvalue (UserInterface|CreateWidget "/Game/Blueprint/Blueprints/Widget/WBP_HUD.WBP_HUD_C"))
    (UserInterface|Viewport|AddtoViewport _returnvalue 0)
    (Variables|Default|SetbIsMainMenu false)
    (Widget|SetVisibility _returnvalue "Hidden")
    (Input|SetInputModeGameOnly self false)
    (else
      (bind _returnvalue_2 (UserInterface|CreateWidget "/Game/Blueprint/Blueprints/Widget/WBP_HUD.WBP_HUD_C"))
      (UserInterface|Viewport|AddtoViewport _returnvalue_2 0)
      (Variables|Default|SetbIsMainMenu true)
      (Widget|SetVisibility _returnvalue_2 "Visible")
      (Variables|/Script/Engine.PlayerController|SetbShowMouseCursor (Game|GetPlayerController 0) true)
      (Input|SetInputModeUIOnly self (Variables|Default|GetHUD) "DoNotLock" false))))

(event Custom|LoadEndGameWidgetClass
  (params (Won :type Boolean))
  ;[0.2308 1 0.1369] Load End Game Widget Class with Async
  (Utilities|AsyncLoadClassAsset (Variables|Default|GetEndGameWidgetClass)
    (:Completed
      (CallFunction|CreateEndGameMenu Won))))

(event Custom|AssignToEndMenuDelegates
  ;[0.2308 1 0.1369] Assign Callbacks to Event Dispatchers
  (bind _endgamewidget (Variables|Default|GetEndGameWidget)
    (:then
      (EventDispatchers|AssignOnQuitGame _endgamewidget (delegate Custom|OnQuitGame_Event))
      (EventDispatchers|AssignOnRestart (Variables|Default|GetEndGameWidget) (delegate Custom|OnRestart_Event)))
    (:else)))

(event Custom|OnQuitGame_Event
  ;[0.2308 1 0.1369] Assign Callbacks to Event Dispatchers
  (Game|QuitGame 0 "Quit" false))

(event Custom|OnRestart_Event
  ;[0.2308 1 0.1369] Assign Callbacks to Event Dispatchers
  (Input|SetInputModeGameOnly (Game|GetPlayerController 0) false)
  (Variables|Default|SetbShowMouseCursor false)
  (Game|OpenLevel(byObjectReference) "/Game/Maps/PrototypeLevel.PrototypeLevel"))

(event Input|EnhancedActionEvents|EnhancedInputActionIA_Look
  (params (ActionValue :type Vector%202D%20Structure) (ElapsedSeconds :type Float%20%28double-precision%29) (TriggeredSeconds :type Float%20%28double-precision%29) (InputAction :type Input%20Action%20Object%20Reference :default "/Game/Input/IA_Look.IA_Look"))
  ;[0.2308 1 0.1369] Look and Move
  (KiksInput|HandleLookatMovement ActionValue))

(event Input|EnhancedActionEvents|EnhancedInputActionIA_Movement
  (params (ActionValue :type Vector%202D%20Structure) (ElapsedSeconds :type Float%20%28double-precision%29) (TriggeredSeconds :type Float%20%28double-precision%29) (InputAction :type Input%20Action%20Object%20Reference :default "/Game/Input/IA_Movement.IA_Movement"))
  ;[0.2308 1 0.1369] Look and Move
  (KiksInput|HandleMovement))

(event Input|EnhancedActionEvents|EnhancedInputActionIA_Jump
  (params (ActionValue :type Boolean) (ElapsedSeconds :type Float%20%28double-precision%29) (TriggeredSeconds :type Float%20%28double-precision%29) (InputAction :type Input%20Action%20Object%20Reference :default "/Game/Input/IA_Jump.IA_Jump"))
  ;[0.2308 1 0.1369] Handle Jump
  (bind _controlledcharacter (Variables|EssentialVariables|GetControlledCharacter)
    (:then
      (Character|Jump _controlledcharacter))
    (:else)))

(event Input|EnhancedActionEvents|EnhancedInputActionIA_Jetpack
  (params (ActionValue :type Boolean) (ElapsedSeconds :type Float%20%28double-precision%29) (TriggeredSeconds :type Float%20%28double-precision%29) (InputAction :type Input%20Action%20Object%20Reference :default "/Game/Input/IA_Jetpack.IA_Jetpack"))
  ;[0.1666 0.9901 1] Start Jetpack Thrusters and set Movement Mode to Flying on Started
  (:Triggered
    ;;[1 0 0] If PC Has Fuel, Apply Thrust and Drain Fuel, otherwisw Stop Jetpack
    (bind _bhasfuel (Class|BPIJetpack|HasFuel(Message) (Variables|EssentialVariables|GetControlledCharacter)))
    (if _bhasfuel
      (Jetpack|ApplyThrusterUpward)
      (Jetpack|DrainJetFuel)
      (else
        (Utilities|FlowControl|DoOnce false
          (:Completed
            (Jetpack|StopJetpack))))))
  (:Started
    ;;[1 0 0] If PC Has Fuel Start Jet Pack
    (bind _bhasfuel_2 (Class|BPIJetpack|HasFuel(Message) (Variables|EssentialVariables|GetControlledCharacter)))
    (if _bhasfuel_2
      (Jetpack|StartJetpack)
      (CallFunction|ResetJetpack)))
  (:Completed
    ;;[1 0 0] Stop Jetpack
    (if (Variables|Default|GetbJetpackActive)
      (Jetpack|StopJetpack))))

(event EventBeginPlay
  ;[0.2308 1 0.1369] Events at Begin play with referances
  (KiksInput|MappingContext)
  (EssentialVariables|StoreMovementComponent)
  (CallFunction|HandleHUD))

(event EventTick
  (params (DeltaSeconds :type Float%20%28single-precision%29))
  ;[0.2308 1 0.1369] On Tick Get Referance to Player Character/ Set Target Arm Length to an Interpolation of Float
  (CameraEssentials|SetTargetArmLength DeltaSeconds))

(event Input|MouseEvents|MouseWheelAxis
  (params (AxisValue :type Float%20%28single-precision%29))
  ;[0.2308 1 0.1369] Zoom IN and OUT with Spring Arm
  (CameraEssentials|PositiveCameraPosition (< AxisValue 0.0))
  (CameraEssentials|NegativeCameraPosition (> AxisValue 0.0)))

(fn ConstructionScript)

(fn HandleLookatMovement
  (params (InVec :type Vector%202D%20Structure))
  (bind (_x _y) (Math|Vector2D|BreakVector2D InVec))
  ;[0.1666 0.9901 1] Handle Player Look
  (Class|PlayerController|AddYawInput _x)
  (Class|PlayerController|AddPitchInput _y))

(fn MoveFowardDirection
  (return (Pawn|GetMovementComponent (Pawn|GetControlledPawn)) (* (Math|Vector|GetForwardVector (Pawn|GetControlRotation :!class /Script/Engine.Controller)) (.y (Input|EnhancedActionValues|GetIA_Movement)))))

(fn MoveRightDirection
  (return (Pawn|GetMovementComponent (Pawn|GetControlledPawn)) (* (Math|Vector|GetRightVector (Pawn|GetControlRotation :!class /Script/Engine.Controller)) (.x (Input|EnhancedActionValues|GetIA_Movement)))))

(fn HandleMovement
  (bind (_movementcomponent _yaxis) (KiksInput|MoveFowardDirection))
  (bind (_movementcomponent_2 _xaxis) (KiksInput|MoveRightDirection))
  ;[0.1666 0.9901 1] Move Player Character
  (Variables|EssentialVariables|GetControlledCharacter
    (:then
      (Class|PawnMovementComponent|AddInputVector _movementcomponent _yaxis false)
      (Class|PawnMovementComponent|AddInputVector _movementcomponent_2 _xaxis false))
    (:else)))

(fn MappingContext
  ;[0.1666 0.9901 1] Handle  Mapping Context
  (Input|AddMappingContext (PlayerController|LocalPlayerSubsystems|GetEnhancedInputLocalPlayerSubsystem) "/Game/Input/IMC_KikMovement.IMC_KikMovement" 0 "(bIgnoreAllPressedKeysUntilRelease=True,bForceImmediately=False,bNotifyUserSettings=False)"))

(fn StoreMovementComponent
  ;[0.1666 0.9901 1] Referances to Player Character and Movement Component
  (bind _ascharacter (Utilities|Casting|CastToCharacter (Pawn|GetControlledPawn)))
  (Variables|EssentialVariables|SetControlledCharacter _ascharacter)
  (bind _ascharacter_movement_component (Utilities|Casting|CastToCharacterMovementComponent (Pawn|GetMovementComponent (Pawn|GetControlledPawn))))
  (Variables|EssentialVariables|SetCharacterMovementComponent _ascharacter_movement_component))

(fn SetTargetArmLength
  (params (DeltaTime :type Float%20%28double-precision%29))
  ;[0.1666 0.9901 1] Cast to Player Character Get Spring Arm Set Spring Arm to Get of Arm Length which wil interpolate Delta seconds with simple math of * between Camera Pos and Camera Zoom Differance then + Spring Arm Default Length
  (bind _asbp_kik (Utilities|Casting|CastToBP_Kik (Game|GetPlayerCharacter 0)))
  (Variables|/Script/Engine.SpringArmComponent|SetTargetArmLength (Variables|/Game/Blueprint/Kik/BP_Kik.BP_Kik_C|GetSpringArm _asbp_kik) (Math|Interpolation|FInterpTo (Variables|/Script/Engine.SpringArmComponent|GetTargetArmLength (Variables|/Game/Blueprint/Kik/BP_Kik.BP_Kik_C|GetSpringArm _asbp_kik)) (+ (Variables|Default|GetSpringArmDefaultLength) (* (Variables|Default|GetCameraZoomDifferance) (Variables|Default|GetCameraPosition))) DeltaTime 2.0)))

(fn PositiveCameraPosition
  (params (Condition :type Boolean))
  (bind _maxcameraposition (Variables|Default|GetMaxCameraPosition))
  ;[0.1666 0.9901 1] If True (condition > 0) decrement Max Camera Pos and Set it on a Clamp between -1 and Max Camera Pos
  (if Condition
    (bind _result (Math|Integer|IncrementInt (Variables|Default|GetMaxCameraPosition))
      (:%20%20
        (Variables|Default|SetCameraPosition (Math|Integer|Clamp(Integer) _result (* _maxcameraposition -1) _maxcameraposition))))))

(fn NegativeCameraPosition
  (params (Condition :type Boolean))
  (bind _maxcameraposition (Variables|Default|GetMaxCameraPosition))
  ;[0.1666 0.9901 1] If True (Condition > 0) decrement Max Camera Pos and Set it on a Clamp between -1 and Max Camera Pos
  (if Condition
    (bind _result (Math|Integer|DecrementInt (Variables|Default|GetMaxCameraPosition))
      (:%20%20
        (Variables|Default|SetCameraPosition (Math|Integer|Clamp(Integer) _result (* _maxcameraposition -1) _maxcameraposition))))))

(fn StartMovementModeFlying
  (bind _charactermovementcomponent (Variables|EssentialVariables|GetCharacterMovementComponent))
  ;[0.1666 0.9901 1] Set Movement Mode from Walking to Fluing and Orient controller to Desired Rotation @ 1440 on the Z
  (Pawn|Components|CharacterMovement|SetMovementMode (Variables|EssentialVariables|GetCharacterMovementComponent) "MOVE_Flying" 0)
  (Variables|/Script/Engine.CharacterMovementComponent|SetbOrientRotationToMovement _charactermovementcomponent false)
  (Variables|/Script/Engine.CharacterMovementComponent|SetbUseControllerDesiredRotation _charactermovementcomponent true))

(fn StartMovementModeWalking
  (bind _charactermovementcomponent (Variables|EssentialVariables|GetCharacterMovementComponent))
  ;[0.1666 0.9901 1] Return Movement Mode to the Original State of Walking
  (Pawn|Components|CharacterMovement|SetMovementMode (Variables|EssentialVariables|GetCharacterMovementComponent) "MOVE_Walking" 0)
  (Variables|/Script/Engine.CharacterMovementComponent|SetbOrientRotationToMovement _charactermovementcomponent true)
  (Variables|/Script/Engine.CharacterMovementComponent|SetbUseControllerDesiredRotation _charactermovementcomponent false))

(fn ApplyThrusterUpward
  ;[0.1666 0.9901 1] Get Character Actor Up Vector and Multiply by .25, Add Input Vector on Character Movement Component
  (bind _controlledcharacter (Variables|EssentialVariables|GetControlledCharacter)
    (:then
      (bind _charactermovementcomponent (Variables|EssentialVariables|GetCharacterMovementComponent)
        (:then
          (Class|PawnMovementComponent|AddInputVector _charactermovementcomponent (* (Transformation|GetActorUpVector _controlledcharacter) (Variables|Default|GetThrustInputVector)) false))
        (:else)))
    (:else)))

(fn StartJetpack
  ;[0.1666 0.9901 1] Stratup Jetpack
  (Variables|Default|SetbJetpackActive true)
  (bind _controlledcharacter (Variables|EssentialVariables|GetControlledCharacter)
    (:then
      (Class|BPIJetpack|StartThruster(Message) _controlledcharacter)
      (Movemnet|StartMovementModeFlying))
    (:else)))

(fn StopJetpack
  ;[0.1666 0.9901 1] Stopping the Jetpack
  (Variables|Default|SetbJetpackActive false)
  (bind _controlledcharacter (Variables|EssentialVariables|GetControlledCharacter)
    (:then
      (Class|BPIJetpack|StopThruster(Message) _controlledcharacter)
      (Movemnet|StartMovementModeWalking))
    (:else)))

(fn DrainJetFuel
  (bind _controlledcharacter (Variables|EssentialVariables|GetControlledCharacter)
    (:then
      (bind _currentfuelpercent (Class|BPIJetpack|DrainJetFuel(Message) _controlledcharacter))
      (Default|FuelAmount (Variables|Default|GetHUD) _currentfuelpercent))
    (:else)))

(fn HandleWidget)

(fn HandleHUD
  ;[1 1 1] If IsMainMenu True Show Player HUD
  (if (Variables|Default|GetbIsMainMenu)
    (bind _returnvalue (UserInterface|CreateWidget "/Game/Blueprint/Blueprints/Widget/WBP_HUD.WBP_HUD_C"))
    (bind _output_get (Variables|Default|SetHUD _returnvalue))
    (UserInterface|Viewport|AddtoViewport _output_get 0)))

(fn FuelUpdate
  (params (FuelPercent :type Float%20%28double-precision%29))
  (|CallParentFunction FuelPercent)
  (bind _hud (Variables|Default|GetHUD)
    (:then
      (Default|FuelAmount _hud FuelPercent))
    (:else)))

(fn ShowEndGameWidget
  (params (Won :type Boolean))
  ;[0.2308 1 0.1369] Display End Game Widget IF IsValidClass True/IF False Load End Game Widget Class
  (|CallParentFunction Won)
  (if (Utilities|IsValidClass (Utilities|ResolveSoftReference (Variables|Default|GetEndGameWidgetClass)))
    (CallFunction|CreateEndGameMenu Won)
    (else
      (CallFunction|LoadEndGameWidgetClass Won))))

(fn GetEndGameText
  (params (Won :type Boolean))
  (if Won
    (return "Winner!!")
    (else
      (return "Loser!!"))))

(fn CreateEndGameMenu
  (params (Won :type Boolean))
  ;[0.2308 1 0.1369] Create End Game Menu Screen
  (bind _returnvalue (UserInterface|CreateWidget (Utilities|ResolveSoftReference (Variables|Default|GetEndGameWidgetClass))))
  (bind _output_get (Variables|Default|SetEndGameWidget _returnvalue))
  (UserInterface|Viewport|AddtoViewport _output_get 0)
  (Default|SetMenuText (Variables|Default|GetEndGameWidget) (CallFunction|GetEndGameText Won))
  (Default|SetPositiontoCenter (Variables|Default|GetEndGameWidget))
  (Input|SetInputModeUIOnly self (Variables|Default|GetEndGameWidget) "DoNotLock" true)
  (Variables|Default|SetbShowMouseCursor true)
  (CallFunction|AssigntoEndMenuDelegates))

(fn DrainJetFuel
  (return 0.0))

(fn GetActionInput
  (return ""))

(fn HasFuel
  (return false))

(fn NoFuel
  (return false))