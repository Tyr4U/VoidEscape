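; Blaster shot projectile in the Drone folder that damages its target character on impact.
; On BeginPlay it binds the Beam component's hit event, which passes the hit result and other actor to HandleBeamHit.
; HandleBeamHit spawns a Niagara burst oriented to the surface normal, applies a small fixed damage only if the hit actor is TargetCharacter, then destroys the shot on any hit.
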(event Custom|OnComponentHit_Event
  (params (HitComponent :type Primitive%20Component%20Object%20Reference) (OtherActor :type Actor%20Object%20Reference) (OtherComp :type Primitive%20Component%20Object%20Reference) (NormalImpulse :type Vector) (Hit :type Hit%20Result%20Structure%20%28by%20ref%29))
  ;[0.2308 1 0.1369] Event Begin Play Events
  (CallFunction|HandleBeamHit Hit OtherActor))

(event EventBeginPlay
  ;[0.2308 1 0.1369] Event Begin Play Events
  (Collision|AssignOnComponentHit (Variables|Default|GetBeam) (delegate Custom|OnComponentHit_Event)))

(fn ConstructionScript)

(fn HandleBeamHit
  (params (Hit :type Hit%20Result%20Structure%20%28by%20ref%29) (HitActor :type Actor%20Object%20Reference))
  (bind (_bblockinghit _binitialoverlap _time _distance _location _impactpoint _normal) (Collision|BreakHitResult Hit))
  (Niagara|SpawnSystematLocation "/Game/Drone/VFX/NS_Burst.NS_Burst" _impactpoint (Math|Rotator|MakeRotfromX _normal))
  ;[1 0 0] Check IF Actor is HIT. IF True do damage system to death
  (if (== (Variables|Default|GetTargetCharacter) HitActor)
    (Game|Damage|ApplyDamage (Variables|Default|GetTargetCharacter) 0.25 0 0))
  (Actor|DestroyActor))